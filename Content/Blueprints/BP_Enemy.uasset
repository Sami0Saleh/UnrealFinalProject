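; Side-to-side moving enemy that takes a Goomba or Mushroom form based on EnemyType, which sets its mesh on BeginPlay.
; Tick drives movement along MoveDirection: Goombas at constant input, Mushrooms by MovementScale, which is set when a player overlaps Detection.
; Any body hit flips direction along X, and a player hit sends OnPlayerHitMessage through BPI_Player, guarded by DoOnce.
; A player hitting the Box component destroys the enemy.
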(event OnComponentHit(Box)
  (params (HitComponent :type Primitive%20Component%20Object%20Reference) (OtherActor :type Actor%20Object%20Reference) (OtherComp :type Primitive%20Component%20Object%20Reference) (NormalImpulse :type Vector :default "0, 0, 0") (Hit :type Hit%20Result%20Structure%20%28by%20ref%29))
  (if (Utilities|DoesObjectImplementInterface OtherActor "/Game/Blueprints/BPI_Player.BPI_Player_C")
    (Variables|Default|SetPlayer OtherActor)
    (Actor|DestroyActor)))

(event OnComponentBeginOverlap(Detection)
  (params (OverlappedComponent :type Primitive%20Component%20Object%20Reference) (OtherActor :type Actor%20Object%20Reference) (OtherComp :type Primitive%20Component%20Object%20Reference) (OtherBodyIndex :type Integer) (bFromSweep :type Boolean) (SweepResult :type Hit%20Result%20Structure%20%28by%20ref%29))
  (if (Utilities|DoesObjectImplementInterface OtherActor "/Game/Blueprints/BPI_Player.BPI_Player_C")
    (Variables|Default|SetPlayer OtherActor)
    (switch Utilities|FlowControl|Switch|SwitchonE_EnemyType (Variables|Default|GetEnemyType)
      (:NewEnumerator1
        (Variables|Default|SetMovement%20Scale 0.5)))))

(event Custom|Direction
  ;[1 1 1] ChangeDirection
  (Utilities|FlowControl|FlipFlop
    (:A
      (Variables|Default|SetMoveDirection "1.000000,0.000000,0.000000"))
    (:B
      (Variables|Default|SetMoveDirection "-1.000000,0.000000,0.000000"))))

(event EventBeginPlay
  (switch Utilities|FlowControl|Switch|SwitchonE_EnemyType (Variables|Default|GetEnemyType)
    (:NewEnumerator0
      (Components|SkeletalMesh|SetSkeletalMeshAsset (Variables|Character|GetMesh) "/Game/Imports/Assets/Goomba/Goomba.Goomba"))
    (:NewEnumerator1
      (Components|StaticMesh|SetStaticMesh (Variables|Default|GetStaticMesh) "/Game/Imports/Assets/Mushroom/Mushroom_g_pCube5.Mushroom_g_pCube5"))))

(event EventTick
  (params (DeltaSeconds :type Float%20%28single-precision%29))
  (switch Utilities|FlowControl|Switch|SwitchonE_EnemyType (Variables|Default|GetEnemyType)
    (:NewEnumerator0
      (Pawn|Input|AddMovementInput (Variables|Default|GetMoveDirection) 0.5 false))
    (:NewEnumerator1
      (Pawn|Input|AddMovementInput (Variables|Default|GetMoveDirection) (Variables|Default|GetMovement%20Scale) false))))

(event Collision|EventHit
  (params (MyComp :type Primitive%20Component%20Object%20Reference) (Other :type Actor%20Object%20Reference) (OtherComp :type Primitive%20Component%20Object%20Reference) (bSelfMoved :type Boolean) (HitLocation :type Vector :default "0, 0, 0") (HitNormal :type Vector :default "0, 0, 0") (NormalImpulse :type Vector :default "0, 0, 0") (Hit :type Hit%20Result%20Structure%20%28by%20ref%29))
  (bind _hitactor (|CollapseGraph Hit))
  (if (Utilities|DoesObjectImplementInterface _hitactor "/Game/Blueprints/BPI_Player.BPI_Player_C")
    (bind _output_get (Variables|Default|SetPlayer _hitactor))
    (Utilities|FlowControl|DoOnce false
      (:Completed
        (Class|BPIPlayer|OnPlayerHit(Message) _output_get))))
  (CallFunction|Direction))

(fn ConstructionScript)