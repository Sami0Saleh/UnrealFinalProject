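; Mario-style block actor that acts as either a breakable brick or a coin-giving question-mark block, choosing its mesh on BeginPlay from PlatformType.
; Overlaps from BPI_Player actors trigger a timeline-driven vertical nudge.
; Bricks then spawn a Niagara break effect and destroy themselves.
; Question blocks spawn animated coins while counting down health, switch to a hit material on the last one, and message the player on every hit, even when empty.
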(event OnComponentBeginOverlap(BoxCollidor)
  (params (OverlappedComponent :type Primitive%20Component%20Object%20Reference) (OtherActor :type Actor%20Object%20Reference) (OtherComp :type Primitive%20Component%20Object%20Reference) (OtherBodyIndex :type Integer) (bFromSweep :type Boolean) (SweepResult :type Hit%20Result%20Structure%20%28by%20ref%29))
  (if (Utilities|DoesObjectImplementInterface OtherActor "/Game/Blueprints/BPI_Player.BPI_Player_C")
    (bind _output_get (Variables|Default|SetPlayer OtherActor))
    (Utilities|IsValid _output_get
      (:Is%20Valid
        (switch Utilities|FlowControl|Switch|SwitchonE_PlatformType (Variables|Default|GetPlatformType)
          (:NewEnumerator0
            (CallFunction|KillBrickBlock))
          (:NewEnumerator1
            (CallFunction|HitQmark)))))))

(event Custom|BrickNodge
  (bind _default_block_height (Variables|Default|GetDefault%20Block%20Height))
  ;[1 1 1] BrickNodge
  (Utilities|FlowControl|Delay 0.1)
  (bind _blocknodge (Timeline|Timeline PlayFromStart)
    (:Update
      (Transformation|SetWorldLocation (Variables|Default|GetCube) (Math|Vector|MakeVector (.x _default_block_height) (.y _default_block_height) (.z (+ _blocknodge (Math|Vector|MakeVector (.x _default_block_height) (.y _default_block_height) (.z _default_block_height))))) false false))))

(event Custom|KillBrickBlock
  ;[1 1 1] Destroing + VFX spawn
  (CallFunction|BrickNodge)
  (Utilities|FlowControl|Delay 0.2)
  (Niagara|SpawnSystematLocation "/Game/VFX/NiagaraSystems/NS_BreakCubes.NS_BreakCubes" (Transformation|GetActorLocation self))
  (Actor|DestroyActor))

(event Custom|HitQmark
  ;[1 1 1] QmarkLogic
  (if (<= (Variables|Default|GetQmarkHealth) 1.0)
    (Utilities|FlowControl|DoOnce false
      (:Completed
        (CallFunction|BrickNodge)
        (CallFunction|CoinSpawn)
        (Rendering|Material|SetMaterial (Variables|Default|GetCube) 0 "/Game/Imports/Assets/Question_mark_box/MM_QmBHitBody.MM_QmBHitBody")))
    (else
      (CallFunction|BrickNodge)
      (Math|Float|DecrementFloat (Variables|Default|GetQmarkHealth)
        (:%20%20
          (CallFunction|CoinSpawn)))))
  (Class|BPIPlayer|CollectCoin(Message) (Variables|Default|GetPlayer)))

(event Custom|CoinNodge
  (bind _default_coin_height (Variables|Default|GetDefault%20Coin%20Height))
  ;[1 1 1] CoinAnim
  (bind _blocknodge (Timeline|Timeline_0 PlayFromStart)
    (:Update
      (Transformation|SetWorldLocation (Variables|/Game/Blueprints/BP_Coin.BP_Coin_C|GetDefaultSceneRoot (Variables|Default|GetCoin)) (Math|Vector|MakeVector (.x _default_coin_height) (.y _default_coin_height) (.z (+ _blocknodge (Math|Vector|MakeVector (.x _default_coin_height) (.y _default_coin_height) (.z _default_coin_height))))) false false))
    (:Finished
      (Actor|DestroyActor (Variables|Default|GetCoin)))))

(event Custom|CoinSpawn
  ;[1 1 1] CoinSpawn
  (bind _returnvalue (Game|SpawnActorfromClass "/Game/Blueprints/BP_Coin.BP_Coin_C" (Math|Transform|MakeTransform (Transformation|GetWorldLocation (Variables|Default|GetCube)) "0.000000,0.000000,90.000000" "1.000000,1.000000,1.000000") "Undefined" "MultiplyWithRoot" 0 0))
  (bind _output_get (Variables|Default|SetCoin _returnvalue))
  (Default|CoinNodge _output_get))

(event EventBeginPlay
  (Variables|Default|SetDefault%20Block%20Height (Transformation|GetWorldLocation (Variables|Default|GetCube)))
  (switch Utilities|FlowControl|Switch|SwitchonE_PlatformType (Variables|Default|GetPlatformType)
    (:NewEnumerator0
      (Components|StaticMesh|SetStaticMesh (Variables|Default|GetCube) "/Game/Imports/Assets/Brick_Block/Brick_Block.Brick_Block"))
    (:NewEnumerator1
      (Components|StaticMesh|SetStaticMesh (Variables|Default|GetCube) "/Game/Imports/Assets/Question_mark_box/Question_Mark_Block_Box005_001.Question_Mark_Block_Box005_001"))))

(event EventTick
  (params (DeltaSeconds :type Float%20%28single-precision%29)))

(fn ConstructionScript)

(fn SetVisual
  (bind _cube (Variables|Default|GetCube))
  (Components|StaticMesh|SetStaticMesh _cube (Variables|Default|GetMesh))
  (Rendering|Material|SetMaterial _cube 0 (Variables|Default|GetMaterial)))