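; BP_FlagPole is a flag pole win trigger that animates its flag when a player reaches it.
; An actor implementing BPI_Player that overlaps the Box prints a debug "win!" string and calls FlagAnim.
; FlagAnim uses DoOnce to play a timeline a single time.
; Each timeline update adds FlagHeight to FlagPart's current world Z, so the offset accumulates rather than setting an absolute height.
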(event OnComponentBeginOverlap(Box)
  (params (OverlappedComponent :type Primitive%20Component%20Object%20Reference) (OtherActor :type Actor%20Object%20Reference) (OtherComp :type Primitive%20Component%20Object%20Reference) (OtherBodyIndex :type Integer) (bFromSweep :type Boolean) (SweepResult :type Hit%20Result%20Structure%20%28by%20ref%29))
  (if (Utilities|DoesObjectImplementInterface OtherActor "/Game/Blueprints/BPI_Player.BPI_Player_C")
    (Development|PrintString "win!")
    (CallFunction|FlagAnim)))

(event Custom|FlagAnim
  (bind _flagpart (Variables|Default|GetFlagPart))
  (bind _returnvalue (Transformation|GetWorldLocation _flagpart))
  ;[1 1 1] FlagAnim
  (Utilities|FlowControl|DoOnce false
    (:Completed
      (bind _flagheight (Timeline|Timeline PlayFromStart)
        (:Update
          (Transformation|SetWorldLocation (Variables|Default|GetFlagPart) (Math|Vector|MakeVector (.x _returnvalue) (.y _returnvalue) (+ _flagheight (.z _returnvalue))) false false))))))

(event EventBeginPlay)

(event Collision|EventActorBeginOverlap
  (params (OtherActor :type Actor%20Object%20Reference)))

(event EventTick
  (params (DeltaSeconds :type Float%20%28single-precision%29)))

(fn ConstructionScript)